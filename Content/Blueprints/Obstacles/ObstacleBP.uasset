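; Obstacle actor that repeatedly changes height by animating the Z scale of its cube through a timeline.
; After a random initial delay, the timeline's Finished output loops it indefinitely, alternating forward and reverse playback via MovingDown, with random pauses between moves.
; DescendingBlock becomes visible as each reverse pass starts and is hidden whenever a pass finishes.
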(event `self.ReceiveBeginPlay`
  (bind (_returnvalue_x _returnvalue_y) (`KismetMathLibrary.BreakVector` (`SceneComponent.K2_GetComponentScale` (`self.1M_Cube`))))
  (`KismetSystemLibrary.Delay` (`KismetMathLibrary.RandomFloatInRange` 3.0 10.0))
  (bind (_direction _newtrack_0) (`Timeline|Timeline_0` :!via `PlayFromStart` :!label _label)
    (:`Update`
      (`SceneComponent.SetWorldScale3D` (`self.1M_Cube`) (`KismetMathLibrary.MakeVector` _returnvalue_x _returnvalue_y _newtrack_0)))
    (:`Finished`
      (`SceneComponent.SetVisibility` (`self.DescendingBlock`) false false)
      (if (`self.movingDown`)
        (`KismetSystemLibrary.Delay` (`KismetMathLibrary.RandomFloatInRange` 5.0 15.0))
        (set `self.MovingDown` false)
        (goto _label :!via `PlayFromStart`)
        (else
          (`KismetSystemLibrary.Delay` (`KismetMathLibrary.RandomFloatInRange` 5.0 15.0))
          (set `self.movingDown` true)
          (`SceneComponent.SetVisibility` (`self.DescendingBlock`) true false)
          (goto _label :!via `ReverseFromEnd`))))))

(fn `UserConstructionScript`)