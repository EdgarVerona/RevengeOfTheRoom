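; Obstacle spawner that scatters a set number of ObstacleBP actors when play begins, if enabled.
; Each gets a random X and Y within plus or minus Radius of the world origin, forming a square area, and sits just below BoundParent's Z.
; Width and depth scales are randomized independently while height scale stays fixed.
; Spawning ignores collisions, so obstacles can overlap.
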(event `self.ReceiveBeginPlay`
  (bind _returnvalue (`KismetMathLibrary.RandomFloatInRange` 1.0 5.0))
  (bind _radius (`self.Radius`))
  (bind _returnvalue_2 (+ _radius 0.0))
  (bind _returnvalue_3 (+ 0.0 (* _radius -1.0)))
  (if (`self.enabled`)
    (for _ (range 1 (+ (`self.Quantity`) 1))
      (`|SpawnActorFromClass` "/Game/Blueprints/Obstacles/ObstacleBP.ObstacleBP_C" (`KismetMathLibrary.MakeTransform` (`KismetMathLibrary.MakeVector` (`KismetMathLibrary.RandomFloatInRange` _returnvalue_3 _returnvalue_2) (`KismetMathLibrary.RandomFloatInRange` _returnvalue_3 _returnvalue_2) (- (.z (.location (`self.GetTransform` (`self.Bound Parent`)))) 1.0)) (struct) (`KismetMathLibrary.MakeVector` _returnvalue _returnvalue 1.0)) "AlwaysSpawn" "OverrideRootScale"))))

(fn `UserConstructionScript`)