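; EnemyOne is a jumping enemy that dies to player projectiles and shoots back at the player.
; A PlayerProjectile hit plays a sound, destroys it, asks its Spawner for another enemy and increments the GameMode score.
; Other hits on a GameTraceChannel2 component trigger a jump if possible, making EnemyOneAI track the player.
; After a delay it spawns an EnemyProjectile offset toward and aimed at the player, with a debug sphere marking the muzzle.
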(event `self.ReceiveHit`
  (params (MyComp :type "PrimitiveComponent Object Reference") (Other :type "Actor Object Reference") (OtherComp :type "PrimitiveComponent Object Reference") (bSelfMoved :type Boolean) (HitLocation :type "Vector Structure") (HitNormal :type "Vector Structure") (NormalImpulse :type "Vector Structure") (Hit :type "HitResult Structure (by ref)"))
  (bind _returnvalue (`self.K2_GetActorLocation` self))
  (bind _returnvalue_2 (`self.K2_GetActorLocation` (`GameplayStatics.GetPlayerCharacter` 0)))
  (bind _returnvalue_3 (+ _returnvalue (`KismetMathLibrary.GreaterGreater_VectorRotator` (100.0 0.0 0.0) (`KismetMathLibrary.FindLookAtRotation` _returnvalue _returnvalue_2))))
  (cast `/Game/Blueprints/Player/PlayerProjectile` Other
    (:`then`
      (`GameplayStatics.SpawnSoundAtLocation` "/Game/Audio/ouch.ouch" (`self.K2_GetActorLocation`))
      (`self.K2_DestroyActor`)
      (`/Game/Blueprints/EnemyOne/EnemyOneSpawner.SpawnEnemy` (`self.Spawner`))
      (bind _asgame_mode (cast `/Game/Blueprints/GameMode` (`GameplayStatics.GetGameMode`)))
      (`/Game/Blueprints/GameMode.Increment Score` _asgame_mode))
    (:`CastFailed`
      (`/Engine/EditorBlueprintResources/StandardMacros.IsValid` Other
        (:`Is Valid`
          (if (and (`self.CanJump`) (`|EnumEquality` (`PrimitiveComponent.GetCollisionObjectType` OtherComp) "ECC_GameTraceChannel2"))
            (`GameplayStatics.SpawnSoundAtLocation` "/Game/Audio/poing.poing" (`self.K2_GetActorLocation`))
            (`self.Jump`)
            (`|ExecutionSequence`
              (:`then_0`
                (bind _returnvalue_4 (`AIBlueprintHelperLibrary.GetAIController` self))
                (bind _asenemy_one_ai (cast `/Game/Blueprints/EnemyOne/EnemyOneAI` _returnvalue_4))
                (`/Game/Blueprints/EnemyOne/EnemyOneAI.TrackPlayer` _asenemy_one_ai))
              (:`then_1`
                (`KismetSystemLibrary.Delay` 1.7)
                (`|SpawnActorFromClass` "/Game/Blueprints/EnemyOne/EnemyProjectile.EnemyProjectile_C" (`KismetMathLibrary.MakeTransform` _returnvalue_3 (`KismetMathLibrary.FindLookAtRotation` _returnvalue_3 _returnvalue_2)) "AlwaysSpawn" "OverrideRootScale")
                (`KismetSystemLibrary.DrawDebugSphere` _returnvalue_3 100.0 12 (struct :`R` 0.031642 :`G` 0.060844 :`B` 1.0 :`A` 1.0) 2.0 2.0)))))))))

(fn `UserConstructionScript`)