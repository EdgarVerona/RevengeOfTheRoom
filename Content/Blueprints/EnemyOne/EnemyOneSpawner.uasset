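; EnemyOneSpawner is a spawner actor that creates an EnemyOne when play begins.
; SpawnEnemy picks random X and Y within plus or minus Radius of the world origin, just below the spawner's own height.
; It assigns itself as the new enemy's Spawner, then calls itself recursively if that reference is invalid, effectively retrying failed spawns.
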(event `self.ReceiveBeginPlay`
  (`self.SpawnEnemy`))

(fn `SpawnEnemy`
  (bind _radius (`self.Radius`))
  (bind _returnvalue (+ _radius 0.0))
  (bind _returnvalue_2 (+ 0.0 (* _radius -1.0)))
  (bind _returnvalue_3 (`|SpawnActorFromClass` "/Game/Blueprints/EnemyOne/EnemyOne.EnemyOne_C" (`KismetMathLibrary.MakeTransform` (`KismetMathLibrary.MakeVector` (`KismetMathLibrary.RandomFloatInRange` _returnvalue_2 _returnvalue) (`KismetMathLibrary.RandomFloatInRange` _returnvalue_2 _returnvalue) (- (.z (.location (`self.GetTransform`))) 1.0))) "Undefined" "OverrideRootScale"))
  (bind _output_get (set `/Game/Blueprints/EnemyOne/EnemyOne.Spawner` self _returnvalue_3))
  (`/Engine/EditorBlueprintResources/StandardMacros.IsValid` _output_get
    (:`Is Not Valid`
      (`self.SpawnEnemy`))))

(fn `UserConstructionScript`)