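; AI controller meant to make its pawn orbit the player character.
; A looping timer increments and prints a heading angle each step.
; Every tick it issues a move without pathfinding to the player's location plus a fixed-length offset rotated by that heading, using the player's world position as rotation axis rather than an up vector.
; A rotate-toward-player step exists but is disconnected.
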(event `self.ReceiveBeginPlay`
  (set `self.Distance` 300.0)
  (`KismetSystemLibrary.K2_SetTimer` null "TrackPlayer" (`self.Delay`) true))

(event `TrackPlayer`
  (bind _desiredheading (`self.DesiredHeading`))
  (set `self.DesiredHeading` (+ _desiredheading 1.0))
  (`KismetSystemLibrary.PrintString` (`KismetStringLibrary.Conv_DoubleToString` _desiredheading)))

(event `self.ReceiveTick`
  (params (DeltaSeconds :type "Float (single-precision)"))
  (bind _returnvalue (`self.K2_GetActorLocation` (`GameplayStatics.GetPlayerCharacter` 0)))
  (`self.MoveToLocation` (+ _returnvalue (`KismetMathLibrary.RotateAngleAxis` (`KismetMathLibrary.MakeVector` 0.0 (`self.Distance`)) (`self.DesiredHeading`) _returnvalue)) -1.0 true false))

(fn `UserConstructionScript`)