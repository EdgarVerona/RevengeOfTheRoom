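; Lava Blueprint whose static mesh rises and recedes in a repeating cycle while the actor is enabled at BeginPlay.
; A Rise timeline drives the mesh's absolute world Z, keeping X and Y, and plays forward to rise and in reverse to recede.
; On each finish, a MovingDown flag picks the next direction after a random delay, with a non-spatial incoming or receding sound announcing each move.
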(event `self.ReceiveBeginPlay`
  (bind _staticmeshcomponent (`self.StaticMeshComponent`))
  (bind (_returnvalue_x _returnvalue_y) (`KismetMathLibrary.BreakVector` (`SceneComponent.K2_GetComponentLocation` _staticmeshcomponent)))
  (if (`self.enabled`)
    (set `self.movingDown` false :!label _label)
    (`GameplayStatics.PlaySound2D` "/Game/Audio/lava_incoming.lava_incoming")
    (bind (_direction _upward_movement) (`Timeline|Rise` :!via `PlayFromStart` :!label _label_2)
      (:`Update`
        (`SceneComponent.K2_SetWorldLocation` _staticmeshcomponent (`KismetMathLibrary.MakeVector` _returnvalue_x _returnvalue_y _upward_movement) false false))
      (:`Finished`
        (if (`self.movingDown`)
          (`KismetSystemLibrary.Delay` (`KismetMathLibrary.RandomFloatInRange` 10.0 30.0))
          (goto _label)
          (else
            (`KismetSystemLibrary.Delay` (`KismetMathLibrary.RandomFloatInRange` 10.0 30.0))
            (set `self.movingDown` true)
            (`GameplayStatics.PlaySound2D` "/Game/Audio/lava_receding.lava_receding")
            (goto _label_2 :!via `ReverseFromEnd`)))))))

(fn `UserConstructionScript`)